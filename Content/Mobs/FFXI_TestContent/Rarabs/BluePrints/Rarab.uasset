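; Rarab mob character Blueprint, under test content, with pawn sensing and a toggleable lock-on target marker.
; Tick sets walk speed from IsSprinting, with the slower speed applied while sprinting.
; BeginPlay activates PawnSensing1, while the PawnSensing see-pawn event latches SawPlayer.
; TargetLockedon flip-flops TargetVisual visibility, and DistanceFromPlayerCheck returns the distance to player 0's character.
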(event OnSeePawn(PawnSensing)
  (params (Pawn :type Pawn%20Object%20Reference))
  (Variables|Default|SetSawPlayer true))

(event EventBeginPlay
  (Components|Activation|Activate (Variables|Default|GetPawnSensing1) false))

(event EventTick
  (params (DeltaSeconds :type Float%20%28single-precision%29))
  (bind _charactermovement (Variables|Character|GetCharacterMovement))
  (if (Variables|Default|GetIsSprinting)
    (Variables|/Script/Engine.CharacterMovementComponent|SetMaxWalkSpeed _charactermovement 1.5e+02)
    (else
      (Variables|/Script/Engine.CharacterMovementComponent|SetMaxWalkSpeed _charactermovement 6e+02))))

(event EventTargetLockedon
  (Utilities|FlowControl|FlipFlop
    (:A
      (Development|SetHiddeninGame (Variables|Default|GetTargetVisual) false false))
    (:B
      (Development|SetHiddeninGame (Variables|Default|GetTargetVisual) true false))))

(fn ConstructionScript)

(fn DistancefromPlayerCheck
  (return (Transformation|GetDistanceTo (Game|GetPlayerCharacter 0))))